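; BP_Main is the PaperZD player character for a side-scrolling action game, locked to the Y=0 plane on Tick.
; Input drives movement, coyote-time jumps and knife, axe or bow combo requests to the animation instance.
; Enemy hits cause knockback, while other damage can be randomly dodged; both paths play damage animation and check for death.
; Retriggerable delays track fall time, triggering camera shake after long falls.
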(event Custom|StopMovement
  (Pawn|Components|CharacterMovement|SetMovementMode (Variables|Character|GetCharacterMovement) "MOVE_None" 0))

(event Custom|EnableMovement
  (Pawn|Components|CharacterMovement|SetMovementMode (Variables|Character|GetCharacterMovement) "MOVE_Walking" 0))

(event Custom|DeadCheck
  (if (<= (Variables|Default|GetHealth) 0)
    (Class|PaperZDAnimInstance|JumptoNode (Variables|/Script/PaperZD.PaperZDAnimationComponent|GetAnimInstance (Variables|Default|GetAnimationComponent)) "Dead" "Main")
    (Input|DisableInput 0)))

(event EventOnMovementModeChanged
  (params (PrevMovementMode :type EMovementMode%20Enum :default "MOVE_None") (NewMovementMode :type EMovementMode%20Enum :default "MOVE_None") (PrevCustomMode :type Byte :default 0) (NewCustomMode :type Byte :default 0))
  (if (Utilities|Enum|Equal(Enum) NewMovementMode "MOVE_Falling")
    (Utilities|FlowControl|Sequence
      (:then_0
        (Variables|Default|SetJumpCoyote true)
        (Utilities|FlowControl|RetriggerableDelay 0.1)
        (Variables|Default|SetJumpCoyote false))
      (:then_1
        (Utilities|FlowControl|RetriggerableDelay 0.5)
        (if (AI|Components|NavMovement|IsFalling (Variables|Character|GetCharacterMovement))
          (Variables|Default|SetFallTime 0.5)
          (Utilities|FlowControl|RetriggerableDelay 0.5)
          (if (AI|Components|NavMovement|IsFalling (Variables|Character|GetCharacterMovement))
            (Variables|Default|SetFallTime 1.0)))))))

(event EventOnLanded
  (params (Hit :type Hit%20Result%20Structure%20%28by%20ref%29))
  (if (>= (Variables|Default|GetFallTime) 1.0)
    (Camera|PlayWorldCameraShake "/Game/Character/Main/PaperZD/BP_CameraShake.BP_CameraShake_C" (Transformation|GetActorLocation) 0.0 5e+02)))

(event Game|Damage|EventAnyDamage
  (params (Damage :type Float%20%28single-precision%29) (DamageType :type Damage%20Type%20Object%20Reference) (InstigatedBy :type Controller%20Object%20Reference) (DamageCauser :type Actor%20Object%20Reference))
  (if (not (<= (Math|Random|RandomFloatinRange 0.1 1.0) (Variables|Default|GetDodgeRate)))
    (Class|BPIStateRequest|JumpStateRequest(Message) (Variables|/Script/PaperZD.PaperZDAnimationComponent|GetAnimInstance (Variables|Default|GetAnimationComponent)) "Damaged" "Main")
    (CallFunction|DeadCheck)))

(event EventOnJumped
  (Class|PaperZDAnimInstance|JumptoNode (Variables|/Script/PaperZD.PaperZDAnimationComponent|GetAnimInstance (Variables|Default|GetAnimationComponent)) "Jump_Activated" "Main"))

(event EventOnWalkingOffLedge
  (params (PreviousFloorImpactNormal :type Vector%20%28by%20ref%29 :default "0, 0, 0") (PreviousFloorContactNormal :type Vector%20%28by%20ref%29 :default "0, 0, 0") (PreviousLocation :type Vector%20%28by%20ref%29 :default "0, 0, 0") (TimeDelta :type Float%20%28single-precision%29))
  (Class|PaperZDAnimInstance|JumptoNode (Variables|/Script/PaperZD.PaperZDAnimationComponent|GetAnimInstance (Variables|Default|GetAnimationComponent)) "Jump_Activated" "Main"))

(event Collision|EventHit
  (params (MyComp :type Primitive%20Component%20Object%20Reference) (Other :type Actor%20Object%20Reference) (OtherComp :type Primitive%20Component%20Object%20Reference) (bSelfMoved :type Boolean) (HitLocation :type Vector :default "0, 0, 0") (HitNormal :type Vector :default "0, 0, 0") (NormalImpulse :type Vector :default "0, 0, 0") (Hit :type Hit%20Result%20Structure%20%28by%20ref%29))
  (if (Actor|ActorHasTag Other "Enemy")
    (if (> (.x (Transformation|GetActorForwardVector)) 0.0)
      (Character|LaunchCharacter "-100.000000,0.000000,100.000000" false false)
      (else
        (Character|LaunchCharacter "120.000000,0.000000,120.000000" false false)))
    (Class|BPIStateRequest|JumpStateRequest(Message) (Variables|/Script/PaperZD.PaperZDAnimationComponent|GetAnimInstance (Variables|Default|GetAnimationComponent)) "Damaged" "Main")
    (CallFunction|DeadCheck)))

(event EventTick
  (params (DeltaSeconds :type Float%20%28single-precision%29))
  (bind _returnvalue (Transformation|GetActorLocation))
  (if (!= (.y _returnvalue) 0.0)
    (Transformation|SetActorLocation (Math|Vector|MakeVector (.x _returnvalue) 0.0 (.z _returnvalue)) false false)))

(event Input|ActionEvents|InputActionJump
  (params (Key :type Key%20Structure :default "None"))
  (:Pressed
    (Character|Jump)
    (if (Variables|Default|GetJumpCoyote)
      (Character|LaunchCharacter "0.000000,0.000000,600.000000" false false))))

(event Input|ActionEvents|InputActionLightAttack
  (params (Key :type Key%20Structure :default "None"))
  (:Pressed
    (if (and (and (Variables|Default|GetResetCombo) (not (AI|Components|NavMovement|IsFalling (Variables|Character|GetCharacterMovement)))) (Variables|Ability|GetKnife))
      (Class|BPIComboRequest|RequestCombo(Message) (Variables|/Script/PaperZD.PaperZDAnimationComponent|GetAnimInstance (Variables|Default|GetAnimationComponent)) "NewEnumerator0"))))

(event Input|ActionEvents|InputActionHeavyAttack
  (params (Key :type Key%20Structure :default "None"))
  (:Pressed
    (if (and (and (Variables|Default|GetResetCombo) (not (AI|Components|NavMovement|IsFalling (Variables|Character|GetCharacterMovement)))) (Variables|Ability|GetAxe))
      (Class|BPIComboRequest|RequestCombo(Message) (Variables|/Script/PaperZD.PaperZDAnimationComponent|GetAnimInstance (Variables|Default|GetAnimationComponent)) "NewEnumerator1"))))

(event Input|ActionEvents|InputActionBow
  (params (Key :type Key%20Structure :default "None"))
  (:Pressed
    (if (and (and (and (not (AI|Components|NavMovement|IsFalling (Variables|Character|GetCharacterMovement))) (Variables|Ability|GetBow)) (Variables|Default|GetResetCombo)) (> (Variables|Default|GetArrow) 0))
      (Class|BPIComboRequest|RequestCombo(Message) (Variables|/Script/PaperZD.PaperZDAnimationComponent|GetAnimInstance (Variables|Default|GetAnimationComponent)) "NewEnumerator3"))))

(event Input|AxisEvents|InputAxisMoveRight
  (params (AxisValue :type Float%20%28single-precision%29))
  (Pawn|Input|AddMovementInput "1.000000,0.000000,0.000000" AxisValue false))

(fn ConstructionScript)