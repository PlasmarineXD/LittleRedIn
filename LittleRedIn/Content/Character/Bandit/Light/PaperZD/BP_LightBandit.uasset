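; BP_LightBandit is a 2D PaperZD enemy that chases the player along X, attacks in range and dies when health runs out.
; Observe and AttackRange overlaps with "Main"-tagged actors set detection and range flags.
; Tick polls these to turn and move, jump to Attack after a delay, or play Dead and destroy the actor.
; AnyDamage subtracts health, plays Damaged and briefly disables movement.
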(event OnComponentBeginOverlap(Observe)
  (params (OverlappedComponent :type Primitive%20Component%20Object%20Reference) (OtherActor :type Actor%20Object%20Reference) (OtherComp :type Primitive%20Component%20Object%20Reference) (OtherBodyIndex :type Integer) (bFromSweep :type Boolean) (SweepResult :type Hit%20Result%20Structure%20%28by%20ref%29))
  (if (Actor|ActorHasTag OtherActor "Main")
    (Variables|Default|SetIsDetected true)))

(event OnComponentEndOverlap(Observe)
  (params (OverlappedComponent :type Primitive%20Component%20Object%20Reference) (OtherActor :type Actor%20Object%20Reference) (OtherComp :type Primitive%20Component%20Object%20Reference) (OtherBodyIndex :type Integer))
  (if (Actor|ActorHasTag OtherActor "Main")
    (Variables|Default|SetIsDetected false)))

(event OnComponentBeginOverlap(AttackRange)
  (params (OverlappedComponent :type Primitive%20Component%20Object%20Reference) (OtherActor :type Actor%20Object%20Reference) (OtherComp :type Primitive%20Component%20Object%20Reference) (OtherBodyIndex :type Integer) (bFromSweep :type Boolean) (SweepResult :type Hit%20Result%20Structure%20%28by%20ref%29))
  (if (Actor|ActorHasTag OtherActor "Main")
    (Variables|Default|SetInRanged true)))

(event OnComponentEndOverlap(AttackRange)
  (params (OverlappedComponent :type Primitive%20Component%20Object%20Reference) (OtherActor :type Actor%20Object%20Reference) (OtherComp :type Primitive%20Component%20Object%20Reference) (OtherBodyIndex :type Integer))
  (if (Actor|ActorHasTag OtherActor "Main")
    (Variables|Default|SetInRanged false)))

(event EventTick
  (params (DeltaSeconds :type Float%20%28single-precision%29))
  (bind _returnvalue (Transformation|GetActorForwardVector))
  (bind _returnvalue_2 (>= (.x _returnvalue) 0.0))
  (Utilities|FlowControl|Sequence
    (:then_0
      (if (and (not (Variables|Default|GetInRanged)) (and (Variables|Default|GetIsDetected) (Variables|Default|GetMovable)))
        (bind _asbp_main (Utilities|Casting|CastToBP_Main (Game|GetPlayerCharacter 0)))
        (if (>= (- (.x (Transformation|GetWorldLocation (Variables|/Script/Engine.Character|GetCapsuleComponent _asbp_main))) (.x (Transformation|GetWorldLocation (Variables|Default|GetCapsuleComponent)))) 0.0)
          (if _returnvalue_2
            _
            (else
              (Transformation|SetActorRotation "0, 0, 0")))
          (elif _returnvalue_2
            (Transformation|SetActorRotation "0.000000,180.000000,0.000000")))
        (Pawn|Input|AddMovementInput "1.000000,0.000000,0.000000" (- (.x (Transformation|GetWorldLocation (Variables|/Script/Engine.Character|GetCapsuleComponent _asbp_main))) (.x (Transformation|GetWorldLocation (Variables|Default|GetCapsuleComponent)))) false)))
    (:then_1
      (if (Variables|Default|GetInRanged)
        (if (Variables|Default|GetMovable)
          (Utilities|FlowControl|Delay 0.8)
          (Class|PaperZDAnimInstance|JumptoNode (Variables|/Script/PaperZD.PaperZDAnimationComponent|GetAnimInstance (Variables|Default|GetAnimationComponent)) "Attack" "LightBandit"))))
    (:then_2
      (if (<= (Variables|Stat|GetHealth) 0.0)
        (Variables|Default|SetMovable false)
        (Collision|SetActorEnableCollision self false)
        (Class|PaperZDAnimInstance|JumptoNode (Variables|/Script/PaperZD.PaperZDAnimationComponent|GetAnimInstance (Variables|Default|GetAnimationComponent)) "Dead" "LightBandit")
        (Utilities|FlowControl|Delay 1.0)
        (Actor|DestroyActor)))))

(event Game|Damage|EventAnyDamage
  (params (Damage :type Float%20%28single-precision%29) (DamageType :type Damage%20Type%20Object%20Reference) (InstigatedBy :type Controller%20Object%20Reference) (DamageCauser :type Actor%20Object%20Reference))
  (Variables|Stat|SetHealth (- (Variables|Stat|GetHealth) Damage))
  (Class|PaperZDAnimInstance|JumptoNode (Variables|/Script/PaperZD.PaperZDAnimationComponent|GetAnimInstance (Variables|Default|GetAnimationComponent)) "Damaged" "LightBandit")
  (Variables|Default|SetMovable false)
  (Utilities|FlowControl|Delay 0.5)
  (Variables|Default|SetMovable true))

(fn ConstructionScript)